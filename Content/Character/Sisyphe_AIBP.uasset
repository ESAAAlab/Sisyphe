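; Sisyphe AI character Blueprint that handles ragdoll falls and getting back up, driven every Tick by the IsRagdoll and GetBackUp flags.
; While ragdolled, it blocks player 0's move input, simulates mesh physics and moves the capsule along with the pelvis.
; GetBackUp restores input, repositions the capsule above the pelvis with a fixed rotation, stops simulation, reattaches the mesh and clears itself.
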(event `self.ReceiveActorBeginOverlap`
  (params (OtherActor :type "Actor Object Reference")))

(event `self.ReceiveTick`
  (params (DeltaSeconds :type "Float (single-precision)"))
  (bind _mesh (`self.Mesh`))
  (bind _mesh_2 (`self.Mesh`))
  (`|ExecutionSequence`
    (:`then_0`
      ;[1 1 1] Falling Down
      (if (`self.IsRagdoll?`)
        (`PlayerController.SetIgnoreMoveInput` (`GameplayStatics.GetPlayerController` 0) true)
        (`PrimitiveComponent.SetSimulatePhysics` (`self.CapsuleComponent`) false)
        (`SkeletalMeshComponent.SetAllBodiesBelowSimulatePhysics` _mesh (`SkinnedMeshComponent.GetBoneName` _mesh 0) true)
        (`SceneComponent.K2_SetWorldLocation` (`self.CapsuleComponent`) (+ (`SceneComponent.GetSocketLocation` (`self.Mesh`) (`KismetStringLibrary.Conv_StringToName` (`self.pelvis`))) (0.0 0.0 40.0)) false false)))
    (:`then_1`
      ;[1 1 1] Back Up
      (if (`self.GetBackUp?`)
        (`PlayerController.SetIgnoreMoveInput` (`GameplayStatics.GetPlayerController` 0) false)
        (`PrimitiveComponent.SetSimulatePhysics` (`self.CapsuleComponent`) false)
        (`SceneComponent.K2_SetWorldLocationAndRotation` (`self.CapsuleComponent`) (+ (`SceneComponent.GetSocketLocation` (`self.Mesh`) (`KismetStringLibrary.Conv_StringToName` (`self.pelvis`))) (0.0 0.0 96.0)) (struct :`Yaw` 180.0) false false)
        (`SkeletalMeshComponent.SetAllBodiesBelowSimulatePhysics` _mesh_2 (`SkinnedMeshComponent.GetBoneName` _mesh_2 0) false)
        (`SceneComponent.K2_AttachTo` (`self.Mesh`) (`self.CapsuleComponent`) "None" "KeepRelativeOffset" false)
        (`SceneComponent.K2_SetRelativeLocationAndRotation` (`self.Mesh`) (0.0 0.0 -90.0) (struct :`Yaw` -90.0) false false)
        (set `self.GetBackUp?` false)))))

(fn `UserConstructionScript`)